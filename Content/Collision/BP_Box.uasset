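; BP_Box is a collision-test actor that logs overlap and hit events on its Cube component to the screen.
; Begin overlap, end overlap and hit each print the names of the involved component, other actor and other component, with overlap messages lingering much longer than hit messages.
; On begin overlap, the Cube also hides itself, stops simulating physics and disables its collision, effectively removing it from play.
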(event `self.Cube.OnComponentBeginOverlap`
  (params (OverlappedComponent :type "PrimitiveComponent Object Reference") (OtherActor :type "Actor Object Reference") (OtherComp :type "PrimitiveComponent Object Reference") (OtherBodyIndex :type Integer) (bFromSweep :type Boolean) (SweepResult :type "HitResult Structure (by ref)"))
  (bind _cube (`self.Cube`))
  (`KismetSystemLibrary.PrintString` (`KismetStringLibrary.Concat_StrStr` "Begin Overlapped Component - " (`KismetSystemLibrary.GetDisplayName` OverlappedComponent) ", Other Actor - " (`KismetSystemLibrary.GetDisplayName` OtherActor) ", Other Comp - " (`KismetSystemLibrary.GetDisplayName` OtherComp)) true true (struct :`G` 0.66 :`B` 1.0 :`A` 1.0) 120.0)
  (`SceneComponent.SetVisibility` _cube false false)
  (`PrimitiveComponent.SetSimulatePhysics` _cube false)
  (`PrimitiveComponent.SetCollisionEnabled` _cube "NoCollision"))

(event `self.Cube.OnComponentEndOverlap`
  (params (OverlappedComponent :type "PrimitiveComponent Object Reference") (OtherActor :type "Actor Object Reference") (OtherComp :type "PrimitiveComponent Object Reference") (OtherBodyIndex :type Integer))
  (`KismetSystemLibrary.PrintString` (`KismetStringLibrary.Concat_StrStr` "End Overlapped Component - " (`KismetSystemLibrary.GetDisplayName` OverlappedComponent) ", Other Actor - " (`KismetSystemLibrary.GetDisplayName` OtherActor) ", Other Comp - " (`KismetSystemLibrary.GetDisplayName` OtherComp)) true true (struct :`G` 0.66 :`B` 1.0 :`A` 1.0) 120.0))

(event `self.Cube.OnComponentHit`
  (params (HitComponent :type "PrimitiveComponent Object Reference") (OtherActor :type "Actor Object Reference") (OtherComp :type "PrimitiveComponent Object Reference") (NormalImpulse :type "Vector Structure") (Hit :type "HitResult Structure (by ref)"))
  (`KismetSystemLibrary.PrintString` (`KismetStringLibrary.Concat_StrStr` "Hit Component - " (`KismetSystemLibrary.GetDisplayName` HitComponent) ", Other Actor - " (`KismetSystemLibrary.GetDisplayName` OtherActor) ", Other Comp - " (`KismetSystemLibrary.GetDisplayName` OtherComp)) true true (struct :`G` 0.66 :`B` 1.0 :`A` 1.0) 1.0))

(fn `UserConstructionScript`)